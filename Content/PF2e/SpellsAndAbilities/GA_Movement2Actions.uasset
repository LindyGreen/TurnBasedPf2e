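; GA_Movement2Actions is a Gameplay Ability that moves a turn-based unit along the grid to a clicked tile.
; On activation it marks tiles within an attribute-based path length as reachable and binds player controller click and right-click events.
; Clicking a reachable tile paths the unit there under a loose Ability.IsPerforming tag, which blocks right-click cancel.
; The ability commits only when movement finishes, then registers the new tile through AC_TurnManager and ends.
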(event Custom|CallMove
  (params (TileIndex :type Int%20Point%20Structure))
  (bind _playercontrollerref (Variables|Default|GetPlayerControllerRef))
  (bind _output_get (Variables|Default|SetDestinationIndex TileIndex))
  (if (Utilities|Array|ContainsItem (.TileStates (Utilities|Struct|BreakS_TileData (.Value (Utilities|Map|Find (Variables|/Script/GASLearning.Grid|GetGridTiles (Variables|Default|GetGridRef)) _output_get)))) "IsReachable")
    ;[0.15 0.15 0.15 0.5] UnbindPC buttons
    (EventDispatchers|UnbindEventfromOnTileorActorClicked _playercontrollerref (delegate Custom|CallMove))
    (EventDispatchers|UnbindallEventsfromCallonRMB _playercontrollerref)
    (Default|ClearStatefromTIles (Variables|Default|GetGridRef) "IsReachable")
    (CallFunction|GeneratePath (Variables|Default|GetDestinationIndex))))

(event Custom|OnUnitFinishMove_Event
  (params (Unit :type BP%20Unit%20Object%20Reference))
  (EventDispatchers|UnbindallEventsfromOnUnitFinishMove Unit)
  (Ability|CommitAbility)
  (Class|TurnManagerComponent|SetUnitonGrid (Actor|GetComponentbyClass (Variables|Default|GetGridRef) "/Game/PF2e/Architecture/Combat/AC_TurnManager.AC_TurnManager_C") Unit (Variables|Default|GetDestinationIndex) false)
  (Ability|GameplayEffect|RemoveLooseGameplayTags (Ability|GetAvatarActorfromActorInfo) (GameplayTags|MakeGameplayTagContainerfromTag "(TagName=\"Ability.IsPerforming\")"))
  (Ability|EndAbility)
  (Variables|Default|SetBP_UNITREF_TD 0))

(event Custom|CallToFollowPath
  (params (Path :type Array%20of%20Int%20Point%20Structures))
  (Ability|GameplayEffect|AddLooseGameplayTags (Ability|GetAvatarActorfromActorInfo) (GameplayTags|MakeGameplayTagContainerfromTag "(TagName=\"Ability.IsPerforming\")"))
  (EventDispatchers|AssignOnUnitFinishMove (Variables|Default|GetBP_UNITREF_TD) (EventDispatchers|CreateEvent :!event Custom|OnUnitFinishMove_Event))
  (Default|EventPathFollow (Variables|Default|GetBP_UNITREF_TD) Path))

(event Custom|RMBPressed
  (if (not (GameplayTags|HasTag (GameplayTags|GetOwnedGameplayTags (Ability|GetAbilitySystemComponentfromActorInfo) :!class /Script/GameplayTags.BlueprintGameplayTagLibrary) "(TagName=\"Ability.IsPerforming\")" true))
    (Ability|EndAbility)))

(event Ability|EventOnEndAbility
  (params (bWasCancelled :type Boolean))
  (Class|Grid|ClearStatefromTiles (Variables|Default|GetGridRef) "IsReachable")
  (if bWasCancelled
    _))

(event Ability|EventActivateAbility
  ;[0.15 0.15 0.15 0.5] InitialSetup
  (bind _asbp_unit (Utilities|Casting|CastToBP_Unit (Ability|GetAvatarActorfromActorInfo)))
  (Variables|Default|SetBP_UNITREF_TD _asbp_unit)
  (Variables|Default|SetPlayerControllerRef (.AsPlayer%20Controller%20Turn%20Based (Utilities|Casting|CastToPlayerController_TurnBased (Game|GetPlayerController 0))))
  ;[0.15 0.15 0.15 0.5] BindPCButtons
  (EventDispatchers|BindEventtoOnTileorActorClicked (Variables|Default|GetPlayerControllerRef) (EventDispatchers|CreateEvent :!event Custom|CallMove))
  (EventDispatchers|BindEventtoCallonRMB (Variables|Default|GetPlayerControllerRef) (EventDispatchers|CreateEvent :!event Custom|RMBPressed))
  ;[0.15 0.15 0.15 0.5] Generates Reachables
  (CallFunction|GenerateReachables))

(fn GenerateReachables
  (bind _bp_unitref_td (Variables|Default|GetBP_UNITREF_TD))
  (bind _owningcombatant (Variables|Default|GetOwningCombatant))
  (bind _locationindex (Variables|/Script/GASLearning.Combatant|GetLocationIndex _owningcombatant))
  (Default|ClearStatefromTIles (Variables|Default|GetGridRef) "IsReachable")
  (Utilities|IsValid _owningcombatant
    (:Is%20Valid
      (bind _path (Default|FindPath (Variables|/Game/PF2e/Architecture/Grid/BP_Grid.BP_Grid_C|GetAC_PathfindingReachables (CallFunction|GetGrid)) _locationindex (Utilities|Struct|MakeIntPoint -1 -1) (Variables|/Game/PF2e/Units/BP_Unit.BP_Unit_C|GetAccessibleTiles _bp_unitref_td) 0.0 (LocalVariables|GetMax%20MS) (Math|Float|Truncate (.ReturnValue (Class|AbilitySystemComponent|GetGameplayAttributeValue (Variables|/Script/GASLearning.Combatant|GetAbilitySystemComponent _bp_unitref_td) "(AttributeName=\"MovementSpeed\",Attribute=/Script/GASLearning.CombatAttributeSet:MovementSpeed,AttributeOwner=\"/Script/CoreUObject.Class'/Script/GASLearning.CombatAttributeSet'\")"))) true false))
      (Utilities|Array|RemoveItem _path _locationindex)
      (for _array_element _path
        (Default|AddStatetoTile (Variables|Default|GetGridRef) _array_element "IsReachable")))))

(fn GeneratePath
  (params (Target :type Int%20Point%20Structure))
  (bind _bp_unitref_td (Variables|Default|GetBP_UNITREF_TD))
  (Utilities|IsValid _bp_unitref_td
    (:Is%20Valid
      (bind _path (Default|FindPath (Variables|/Game/PF2e/Architecture/Grid/BP_Grid.BP_Grid_C|GetAC_Pathfinding (CallFunction|GetGrid)) (Variables|/Script/GASLearning.Combatant|GetLocationIndex _bp_unitref_td) Target (Variables|/Game/PF2e/Units/BP_Unit.BP_Unit_C|GetAccessibleTiles _bp_unitref_td) 0.0 (LocalVariables|GetMax%20MS) (Math|Float|Truncate (.ReturnValue (Class|AbilitySystemComponent|GetGameplayAttributeValue (Variables|/Script/GASLearning.Combatant|GetAbilitySystemComponent _bp_unitref_td) "(AttributeName=\"MovementSpeed\",Attribute=/Script/GASLearning.CombatAttributeSet:MovementSpeed,AttributeOwner=\"/Script/CoreUObject.Class'/Script/GASLearning.CombatAttributeSet'\")"))) false true))
      (CallFunction|CalltoFollowPath _path))))