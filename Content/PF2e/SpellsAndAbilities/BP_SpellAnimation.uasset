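; BP_SpellAnimation is a short-lived actor that plays a spell's visual from an origin grid tile to each attacked tile.
; On BeginPlay it spawns a red BP_AnimatedShape per attacked index, using tile transforms from the Grid and binding its completion event.
; It also completes right after the spawn loop without waiting for the shapes, broadcasting OnSpellAnimationCompleted and destroying itself.
; On Destroyed it unbinds only from the last spawned shape.
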(event Custom|Event_PlaySpellAnimation
  (bind _originindex (Variables|Default|GetOriginIndex))
  (bind _transform (CallFunction|GetIndexTransform _originindex))
  (for _array_element (Variables|Default|GetAttackedIndexArray)
    (bind _returnvalue (Game|SpawnActorfromClass "/Game/PF2e/SpellsAndAbilities/Components/BP_AnimatedShape.BP_AnimatedShape_C" (Math|Transform|MakeTransform "0, 0, 0" "0, 0, 0" "1.000000,1.000000,1.000000") "Undefined" "MultiplyWithRoot" 0 (Variables|Default|GetSpellMesh) (Variables|Default|GetMaterial) "(R=1.000000,G=0.000000,B=0.000000,A=1.000000)" (Math|Transform|MakeTransform (.location _transform) (.rotation _transform) "1.000000,1.000000,1.000000") (CallFunction|GetIndexTransform _array_element) 0))
    (EventDispatchers|BindEventtoOnShapeAnimatinCompleted _returnvalue (delegate Custom|CompleteSpellAnimation)))
  (CallFunction|CompleteSpellAnimation))

(event Custom|CompleteSpellAnimation
  (params (NewParam :type Actor%20Object%20Reference))
  (CallFunction|EventCompleteAnimation))

(event Custom|EventCompleteAnimation
  (Default|CallOnSpellAnimationCompleted self)
  (Actor|DestroyActor))

(event EventDestroyed
  ;[0.15 0.15 0.15 0.5] QUESTIONALBLE
  (EventDispatchers|UnbindEventfromOnShapeAnimatinCompleted (stale Custom|Event_PlaySpellAnimation _returnvalue) (delegate Custom|CompleteSpellAnimation)))

(event EventBeginPlay
  (CallFunction|EventPlaySpellAnimation))

(fn ConstructionScript)

(fn GetIndexTransform
  (params (Key :type Int%20Point%20Structure%20%28by%20ref%29))
  (return (Utilities|Struct|BreakS_TileData (.Value (Utilities|Map|Find (Variables|/Game/PF2e/Architecture/Grid/BP_Grid.BP_Grid_C|GetGridTiles (Variables|Default|GetGrid)) Key)))))