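; Gameplay ability for a one-action grid move of the current combatant in a turn-based tactics game.
; On activation it highlights reachable tiles, bounded by a unit attribute, and binds to the player controller's tile-click event.
; Clicking a reachable tile finds a path that the unit follows.
; When movement finishes, it commits the ability, updates the unit's grid position through the turn manager and ends.
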(event Custom|CallMove
  (params (TileIndex :type Int%20Point%20Structure))
  (bind _output_get (Variables|Default|SetDestinationIndex TileIndex))
  (bind _outputtiledata (Default|GetTileDatafromGrid (CallFunction|GetGrid) _output_get))
  (if (Utilities|Array|ContainsItem (.TileStates (Utilities|Struct|BreakS_TileData _outputtiledata)) "IsReachable")
    (EventDispatchers|UnbindEventfromOnTileorActorClicked (.AsPlayer%20Controller%20Turn%20Based (Utilities|Casting|CastToPlayerController_TurnBased (Game|GetPlayerController 0))) (delegate Custom|CallMove))
    (Default|ClearStatefromTIles (CallFunction|GetGrid) "IsReachable")
    (CallFunction|GeneratePath (Variables|Default|GetDestinationIndex))))

(event Custom|OnUnitFinishMove_Event
  (params (Unit :type BP%20Unit%20Object%20Reference))
  (EventDispatchers|UnbindallEventsfromOnUnitFinishMove (Variables|Default|GetBP_UNITREF_TD))
  (Ability|CommitAbility)
  (Class|TurnManagerComponent|SetUnitonGrid (Variables|/Game/PF2e/Architecture/Grid/BP_Grid.BP_Grid_C|GetAC_TurnManager (CallFunction|GetGrid)) Unit (Variables|Default|GetDestinationIndex) false)
  (Ability|EndAbility)
  (Variables|Default|SetBP_UNITREF_TD 0))

(event Custom|CallToFollowPath
  (params (Path :type Array%20of%20Int%20Point%20Structures))
  (bind _bp_unitref_td (Variables|Default|GetBP_UNITREF_TD))
  (Development|PrintString (Utilities|String|Append (Utilities|String|ToString(Text) (Variables|/Script/GASLearning.Combatant|GetCharacterName _bp_unitref_td)) " Called to FollowPath"))
  (EventDispatchers|AssignOnUnitFinishMove (Variables|Default|GetBP_UNITREF_TD) (delegate Custom|OnUnitFinishMove_Event))
  (Default|EventPathFollow _bp_unitref_td Path))

(event Ability|EventActivateAbility
  ;[0.15 0.15 0.15 0.5] InitialSetup
  (bind _returnvalue (Class|MyBaseGameplayAbility|TrySpendActions 1)) ; Action number check
  (if _returnvalue
    (bind _asbp_unit (Utilities|Casting|CastToBP_Unit (Variables|/Script/GASLearning.TurnManagerComponent|GetCurrentCombatant (Variables|/Game/PF2e/Architecture/Grid/BP_Grid.BP_Grid_C|GetAC_TurnManager (CallFunction|GetGrid)))))
    (bind _output_get (Variables|Default|SetBP_UNITREF_TD _asbp_unit))
    (Development|PrintString (Utilities|String|ToString(Text) (Variables|/Script/GASLearning.Combatant|GetCharacterName _output_get)))
    ;[0.15 0.15 0.15 0.5] Binding To MouseClick
    (EventDispatchers|BindEventtoOnTileorActorClicked (.AsPlayer%20Controller%20Turn%20Based (Utilities|Casting|CastToPlayerController_TurnBased (Game|GetPlayerController 0))) (delegate Custom|CallMove))
    ;[0.15 0.15 0.15 0.5] Generates Reachables
    (CallFunction|GenerateReachables)))

(event Ability|EventOnEndAbility
  (params (bWasCancelled :type Boolean))
  (Class|Grid|ClearStatefromTiles (CallFunction|GetGrid) "IsReachable")
  (if bWasCancelled
    _))

(fn GenerateReachables
  (bind _returnvalue (CallFunction|GetGrid))
  (bind _returnvalue_2 (Class|MyBaseGameplayAbility|GetOwningCombatant))
  (bind _bp_unitref_td (Variables|Default|GetBP_UNITREF_TD))
  (bind _locationindex (Variables|/Script/GASLearning.Combatant|GetLocationIndex _returnvalue_2))
  (Default|ClearStatefromTIles _returnvalue "IsReachable")
  (Utilities|IsValid _returnvalue_2
    (:Is%20Valid
      (bind _path (Default|FindPath (Variables|/Game/PF2e/Architecture/Grid/BP_Grid.BP_Grid_C|GetAC_PathfindingReachables _returnvalue) _locationindex (Utilities|Struct|MakeIntPoint -1 -1) (Variables|/Game/PF2e/Units/BP_Unit.BP_Unit_C|GetAccessible%20Tiles _bp_unitref_td) 0.0 (LocalVariables|GetMax%20MS) (Math|Float|Truncate (.ReturnValue (Class|AbilitySystemComponent|GetGameplayAttributeValue (Variables|/Script/GASLearning.Combatant|GetAbilitySystemComponent _bp_unitref_td) "(AttributeName=\"MovementSpeed\",Attribute=/Script/GASLearning.CombatAttributeSet:MovementSpeed,AttributeOwner=\"/Script/CoreUObject.Class'/Script/GASLearning.CombatAttributeSet'\")"))) true false))
      (Utilities|Array|RemoveItem _path _locationindex)
      (for _array_element _path
        (Default|AddStatetoTile (CallFunction|GetGrid) _array_element "IsReachable")))))

(fn GeneratePath
  (params (Target :type Int%20Point%20Structure))
  (bind _bp_unitref_td (Variables|Default|GetBP_UNITREF_TD))
  (Utilities|IsValid _bp_unitref_td
    (:Is%20Valid
      (bind _path (Default|FindPath (Variables|/Game/PF2e/Architecture/Grid/BP_Grid.BP_Grid_C|GetAC_Pathfinding (CallFunction|GetGrid)) (Variables|/Script/GASLearning.Combatant|GetLocationIndex _bp_unitref_td) Target (Variables|/Game/PF2e/Units/BP_Unit.BP_Unit_C|GetAccessible%20Tiles _bp_unitref_td) 0.0 (LocalVariables|GetMax%20MS) (Math|Float|Truncate (* (.ReturnValue (Class|AbilitySystemComponent|GetGameplayAttributeValue (Variables|/Script/GASLearning.Combatant|GetAbilitySystemComponent _bp_unitref_td) "(AttributeName=\"MovementSpeed\",Attribute=/Script/GASLearning.CombatAttributeSet:MovementSpeed,AttributeOwner=\"/Script/CoreUObject.Class'/Script/GASLearning.CombatAttributeSet'\")")) 2.0)) false true))
      (CallFunction|CalltoFollowPath _path))))