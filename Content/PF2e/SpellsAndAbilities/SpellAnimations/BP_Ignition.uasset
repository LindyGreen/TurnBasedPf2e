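; BP_Ignition is the spell animation actor for the Ignition spell in the PF2e game.
; On play, it derives start, end and direction from grid tiles, repositions itself with a height offset, then enables tick and activates ProjectileMovement.
; The arc check only prints debug hit/miss text.
; Tick is empty, and the Timeline that would scale the effect and call CompleteSpellAnimation is unconnected.
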(event EventBeginPlay
  (|CallParentFunction) ; This node is disabled and will not be called.\nDrag off pins to build functionality.
)

(event EventEventPlaySpellAnimation
  (Variables|Default|SetStart (|StartPointVector))
  (Variables|Default|SetEnd (|EndPointVector))
  (Variables|Default|SetDirection (|DirectionVector))
  (bind _newparam (CallFunction|ShouldSpellArc (Variables|Default|GetStart) (Variables|Default|GetEnd) (Variables|Default|GetDirection)))
  (Transformation|SetActorLocationAndRotation (|(({4333EFB0-476E-B0D1-77AF-6C83E91542BE}+({8649F270-4AD5-F796-89C8-8CB5199A9C25}*100))+Height) "0.000000,0.000000,150.000000") "0, 0, 0")
  (if _newparam
    (Development|PrintString "hit")
    (else
      (Development|PrintString "didn't hit")))
  (Actor|Tick|SetActorTickEnabled true)
  (Components|Activation|Activate (Variables|Default|GetProjectileMovement) false))

(event EventTick
  (params (DeltaSeconds :type Float%20%28single-precision%29)))

(fn ConstructionScript
  (|CallParentFunction))