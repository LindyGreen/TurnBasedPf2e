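; BP_GridVisual renders the PF2e grid's tiles, with an optional tactical view.
; It feeds two child BP_GridMeshIns actors shape-specific meshes: flat ones for walkable tiles, and type-colored meshes for the tactical layer.
; Tile updates replace instances by index, stretching tactical tiles vertically by their height above the lowest recorded Z.
; Toggling tactical mode shows or hides that layer and all actors tagged "Tactical".
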(event EventBeginPlay)

(event Collision|EventActorBeginOverlap
  (params (OtherActor :type Actor%20Object%20Reference)))

(event EventTick
  (params (DeltaSeconds :type Float%20%28single-precision%29)))

(fn ConstructionScript)

(fn InitializeGridVisual
  (params (Grid :type BP%20Grid%20Object%20Reference))
  (Variables|Default|SetGrid Grid)
  (Variables|Default|SetGrid%20Mesh%20Ins (.AsBP%20Grid%20Mesh%20Ins (Utilities|Casting|CastToBP_GridMeshIns (Variables|/Script/Engine.ChildActorComponent|GetChildActor (Variables|Default|GetGridMeshInst)))))
  (Variables|Default|SetGrid%20Mesh%20Ins_Tactical (.AsBP%20Grid%20Mesh%20Ins (Utilities|Casting|CastToBP_GridMeshIns (Variables|/Script/Engine.ChildActorComponent|GetChildActor (Variables|Default|GetGridMeshInst_Tactical)))))
  (Utilities|FlowControl|Sequence
    (:then_0
      (Default|InitializeGridMeshInst (Variables|Default|GetGrid%20Mesh%20Ins) "QueryOnly" (.flatmesh (CallFunction|GetShapeData (Variables|/Game/PF2e/Architecture/Grid/BP_Grid.BP_Grid_C|GetTile%20Shape (Variables|Default|GetGrid)))) (.flatmaterial (CallFunction|GetShapeData (Variables|/Game/PF2e/Architecture/Grid/BP_Grid.BP_Grid_C|GetTile%20Shape (Variables|Default|GetGrid)))) false))
    (:then_1
      (Default|InitializeGridMeshInst (Variables|Default|GetGrid%20Mesh%20Ins_Tactical) "QueryOnly" (.mesh (CallFunction|GetShapeData (Variables|/Game/PF2e/Architecture/Grid/BP_Grid.BP_Grid_C|GetTile%20Shape (Variables|Default|GetGrid)))) (.meshmaterial (CallFunction|GetShapeData (Variables|/Game/PF2e/Architecture/Grid/BP_Grid.BP_Grid_C|GetTile%20Shape (Variables|Default|GetGrid)))) true)
      (Variables|Default|SetGridLowestZ 99999.0)
      (CallFunction|SetIsTactical (Variables|Default|GetIs%20Tactical)))))

(fn DestroyGridVisual
  (bind _grid_mesh_ins (Variables|Default|GetGrid%20Mesh%20Ins))
  (Utilities|FlowControl|Sequence
    (:then_0
      (Utilities|IsValid _grid_mesh_ins
        (:Is%20Valid
          (Default|Clearinstances _grid_mesh_ins)
          (return))))
    (:then_1
      (Utilities|IsValid 0
        (:Is%20Valid
          (Default|Clearinstances (Variables|Default|GetGrid%20Mesh%20Ins_Tactical))
          (return))))))

(fn UpdateTileVisual
  (params (TileData :type S%20Tile%20Data%20Structure))
  (Utilities|FlowControl|Sequence
    (:then_0
      (Default|RemoveInstance (Variables|Default|GetGrid%20Mesh%20Ins) (.index TileData))
      (if (CallFunction|IstileTypeWalkable (.tiletype TileData))
        (Default|AddInstance (Variables|Default|GetGrid%20Mesh%20Ins) (.transform TileData) (.index TileData) (.tilestates TileData) (.tiletype TileData))))
    (:then_1
      (CallFunction|UpdateTileVisualTactical TileData))))

(fn UpdateTileVisualTactical
  (params (InputPin :type S%20Tile%20Data%20Structure))
  (bind _grid (Variables|Default|GetGrid))
  (bind (_location _rotation _scale) (Math|Transform|BreakTransform (.transform InputPin)))
  (bind _returnvalue (Default|GetGridTileSize _grid))
  (bind _location_2 (Math|Transform|BreakTransform (.transform InputPin)))
  (Utilities|FlowControl|Sequence
    (:then_0
      (if (< (.z _location_2) (Variables|Default|GetGridLowestZ))
        (Variables|Default|SetGridLowestZ (.z _location_2))))
    (:then_1
      (if (Variables|Default|GetIs%20Tactical)
        (Default|RemoveInstance (Variables|Default|GetGrid%20Mesh%20Ins_Tactical) (.index InputPin))
        (if (Utilities|Enum|NotEqual(Enum) (.tiletype InputPin) "NewEnumerator0")
          (Default|AddInstance (Variables|Default|GetGrid%20Mesh%20Ins_Tactical) (Math|Transform|MakeTransform (Math|Vector|MakeVector (.x _location) (.y _location) (.z _location)) _rotation (Math|Vector|MakeVector (.x _scale) (.y _scale) (/ (+ (- (.Z (Math|Vector|BreakVector (.Location (Math|Transform|BreakTransform (.transform InputPin))))) (Variables|Default|GetGridLowestZ)) (.z _returnvalue)) (.z _returnvalue)))) (.index InputPin) (.tilestates InputPin) (.tiletype InputPin)))))))

(fn SetIsTactical
  (params (bIsTactical :type Boolean))
  (Variables|Default|SetIs%20Tactical bIsTactical)
  (Development|SetHiddeninGame (Variables|Default|GetGridMeshInst_Tactical) (not (Variables|Default|GetIs%20Tactical)) true)
  (bind _outactors (Actor|GetAllActorswithTag "Tactical"))
  (for _array_element _outactors
    (Rendering|SetActorHiddenInGame _array_element (not (Variables|Default|GetIs%20Tactical)))))