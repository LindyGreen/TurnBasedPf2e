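; Deprecated grid actor that draws tiles through one instanced static mesh, with mesh, material and collision set at initialization.
; An array of tile indices mirrors instance order, so tiles are added, replaced or removed by grid index, or cleared together.
; A helper picks colors by tile type or prioritized tile state, but the per-instance custom data writes that would apply them in AddInstance are disconnected.
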(fn ConstructionScript)

(fn AddInstance
  (params (Transform :type Transform%20%28by%20ref%29) (Index :type Int%20Point%20Structure%20%28by%20ref%29) (States :type Array%20of%20ETileState%20Enums :default "None") (TileType :type ETileType%20Enum :default "None"))
  (CallFunction|RemoveInstance Index)
  (Components|InstancedStaticMesh|AddInstance (Variables|Default|GetInstancedStaticMesh) Transform true)
  (bind _returnvalue (Utilities|Array|Add (Variables|Default|GetInstanceIndexes) Index))
  (LocalVariables|SetArrayIndex _returnvalue))

(fn RemoveInstance
  (params (Index :type Int%20Point%20Structure%20%28by%20ref%29))
  (bind _instanceindexes (Variables|Default|GetInstanceIndexes))
  (if (Utilities|Array|ContainsItem _instanceindexes Index)
    (Class|InstancedStaticMeshComponent|RemoveInstance (Variables|Default|GetInstancedStaticMesh) (Utilities|Array|FindItem _instanceindexes Index))
    (Utilities|Array|RemoveItem _instanceindexes Index)))

(fn Clearinstances
  (Components|InstancedStaticMesh|ClearInstances (Variables|Default|GetInstancedStaticMesh))
  (Utilities|Array|Clear (Variables|Default|GetInstanceIndexes)))

(fn InitializeGridMeshInst
  (params (Collision :type ECollisionEnabled%20Enum :default "NoCollision") (Mesh :type Static%20Mesh%20Object%20Reference) (Material :type Material%20Interface%20Object%20Reference) (ColorBasedOnTileType :type Boolean))
  (bind _instancedstaticmesh (Variables|Default|GetInstancedStaticMesh))
  (Components|StaticMesh|SetStaticMesh _instancedstaticmesh Mesh)
  (Rendering|Material|SetMaterial _instancedstaticmesh 0 Material)
  (Variables|Default|SetbIsColorBasedOnTileType ColorBasedOnTileType)
  (Collision|SetCollisionEnabled _instancedstaticmesh Collision))

(fn GetColorfromStateorTile
  (params (TileType :type E_Tiletype_TBD%20Enum :default "NewEnumerator0") (States :type Array%20of%20E_TileState_TOBEDEPRICATED%20Enums :default "NewEnumerator0"))
  (if (Variables|Default|GetbIsColorBasedOnTileType)
    (return (Utilities|Select :Index TileType :NewEnumerator0 "" :NewEnumerator1 "(R=0.958333,G=0.958333,B=0.958333,A=1.000000)" :NewEnumerator2 "(R=0.692708,G=0.000000,B=0.000000,A=1.000000)" :NewEnumerator3 "(R=0.009170,G=0.489583,B=0.191448,A=1.000000)" :NewEnumerator4 "(R=0.000000,G=0.359375,B=0.099508,A=1.000000)" :NewEnumerator5 "(R=0.000000,G=0.072170,B=1.000000,A=1.000000)"))
    (elif (Utilities|Array|IsEmpty States)
      (return "")
      (else
        (for _array_element (Utilities|Array|MakeArray "NewEnumerator9" "NewEnumerator8" "NewEnumerator2" "NewEnumerator1" "NewEnumerator4" "NewEnumerator7")
          (if (Utilities|Array|ContainsItem States _array_element)
            (return (Utilities|Select :Index _array_element :NewEnumerator0 "" :NewEnumerator1 "(R=1.000000,G=0.980678,B=0.000000,A=1.000000)" :NewEnumerator2 "(R=1.000000,G=0.240347,B=0.000000,A=1.000000)" :NewEnumerator3 "(R=1.000000,G=0.000000,B=0.416354,A=1.000000)" :NewEnumerator4 "(R=0.000000,G=1.000000,B=0.522382,A=1.000000)" :NewEnumerator5 "" :NewEnumerator6 "" :NewEnumerator7 "(R=0.000000,G=0.034733,B=0.739000,A=1.000000)" :NewEnumerator8 "(R=0.692708,G=0.025676,B=0.000000,A=1.000000)" :NewEnumerator9 "(R=0.038025,G=1.000000,B=0.000000,A=1.000000)"))))
        (return "")))))