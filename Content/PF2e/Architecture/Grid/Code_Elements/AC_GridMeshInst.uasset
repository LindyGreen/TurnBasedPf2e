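; Grid visual component for the PF2e tactical grid, extending a C++ parent that renders tiles as instanced flat-square meshes.
; InitializeGridVisual stores the grid and sets up the mesh, material and query-only collision.
; ColorTile writes RGBA into per-instance custom data, using a color from GetColorFromStateOrTile.
; That function maps either tile type or the highest-priority tile state to a color, though ColorTile always passes None as type.
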(event EventColorTile
  (params (TileData :type S%20Tile%20Data%20Structure) (AddedIndex :type Integer))
  (bind _instancedmeshcomponent (Variables|Default|GetInstancedMeshComponent))
  (Variables|Default|SetIndexToColor AddedIndex)
  (bind _newparam (CallFunction|GetColorfromStateorTile "None" (.tilestates TileData)))
  (Components|InstancedStaticMesh|SetCustomDataValue _instancedmeshcomponent (Variables|Default|GetIndexToColor) 0 (.r _newparam) true)
  (Components|InstancedStaticMesh|SetCustomDataValue _instancedmeshcomponent (Variables|Default|GetIndexToColor) 1 (.g _newparam) true)
  (Components|InstancedStaticMesh|SetCustomDataValue _instancedmeshcomponent (Variables|Default|GetIndexToColor) 2 (.b _newparam) true)
  (Components|InstancedStaticMesh|SetCustomDataValue _instancedmeshcomponent (Variables|Default|GetIndexToColor) 3 (.a _newparam) true))

(fn GetColorfromStateorTile
  (params (TileType :type ETileType%20Enum :default "None") (States :type Array%20of%20ETileState%20Enums :default "None"))
  (if (Variables|Default|GetbIsColorBasedOnTileType)
    (return (Utilities|Select :Index TileType :None "" :Normal "(R=0.991319,G=0.991319,B=0.991319,A=1.000000)" :Obstacle "(R=1.000000,G=0.000000,B=0.042304,A=1.000000)" :DifficultTerrain "(R=0.388021,G=0.204610,B=0.000000,A=1.000000)" :GreaterDiffTerrain "(R=0.110243,G=0.085987,B=0.000000,A=1.000000)" :FlyOnly "(R=0.000000,G=0.119538,B=1.000000,A=1.000000)"))
    (elif (Utilities|Array|IsEmpty States)
      (return "")
      (else
        (for _array_element (Utilities|Array|MakeArray "IsSpellAOE" "IsInRange" "Selected" "Hovered" "IsInPath" "IsReachable" "None")
          (if (Utilities|Array|ContainsItem States _array_element)
            (return (Utilities|Select :Index _array_element :None "" :Hovered "(R=0.538401,G=1.000000,B=0.000000,A=1.000000)" :Selected "(R=1.000000,G=0.670088,B=0.000000,A=1.000000)" :Neighbor "(R=0.110243,G=0.085987,B=0.000000,A=1.000000)" :IsInPath "(R=0.275174,G=0.029112,B=0.029112,A=1.000000)" :IsDiscovered "" :IsAnalyzed "" :IsReachable "(R=0.000000,G=0.000000,B=1.000000,A=1.000000)" :IsInRange "(R=1.000000,G=0.000000,B=0.000000,A=1.000000)" :IsSpellAOE "(R=0.000000,G=1.000000,B=0.000000,A=1.000000)"))))
        (return "")))))

(fn InitializeGridVisual
  (params (Grid :type BP%20Grid%20Object%20Reference))
  (Variables|Default|SetGrid Grid)
  (Class|GridMeshInstance|InitializeGridMeshInst "/Game/PF2e/Architecture/Grid/Square/SM_Grid_SquareFlat.SM_Grid_SquareFlat" "/Game/PF2e/Architecture/Grid/Square/MI_Grid_Flat_Square.MI_Grid_Flat_Square" "QueryOnly" false))