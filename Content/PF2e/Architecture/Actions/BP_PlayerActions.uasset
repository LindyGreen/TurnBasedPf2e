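; Player input actor that turns cursor hover and mouse clicks on the BP_Grid into tile and unit actions.
; Each tick it resolves the hovered unit or tile, updating hover states and notifying both selected actions.
; Left and right clicks execute swappable spawned action actors, repeating on newly hovered tiles while held.
; It also owns tile and unit selection, with handlers to refresh it on grid or unit index changes.
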(event Custom|OnHoverTileChaged
  (bind _selectedaction_leftclick (Variables|ActionsAndInput|GetSelectedAction_LeftClick))
  (bind _selectedaction_rightclick (Variables|ActionsAndInput|GetSelectedAction_RightClick))
  (bind _hoveredtile (Variables|Default|GetHoveredTile))
  (Utilities|FlowControl|Sequence
    (:then_0
      (bind _selectedaction_leftclick_2 (Variables|ActionsAndInput|GetSelectedAction_LeftClick)
        (:then
          (Default|ExecuteHoveredAction _selectedaction_leftclick_2 _hoveredtile)
          (if (Variables|ActionsandInput|GetbIsLMBHeld)
            (Utilities|IsValid _selectedaction_leftclick
              (:Is%20Valid
                (Default|ExecuteAction _selectedaction_leftclick (Variables|Default|GetHoveredTile))))))
        (:else)))
    (:then_1
      (bind _selectedaction_rightclick_2 (Variables|ActionsAndInput|GetSelectedAction_RightClick)
        (:then
          (Default|ExecuteHoveredAction _selectedaction_rightclick_2 _hoveredtile)
          (if (Variables|ActionsandInput|GetbIsRMBHeld)
            (Utilities|IsValid _selectedaction_rightclick
              (:Is%20Valid
                (Default|ExecuteAction _selectedaction_rightclick (Variables|Default|GetHoveredTile))))))
        (:else)))))

(event EventBeginPlay
  ;[0.15 0.15 0.15 0.5] Refactor
  (bind _returnvalue (Actor|GetActorOfClass "/Game/PF2e/Architecture/Grid/BP_Grid.BP_Grid_C"))
  (Variables|Default|SetBP_Grid _returnvalue)
  (EventDispatchers|BindEventtoOnGridGenerated (Variables|Default|GetBP_Grid) (EventDispatchers|CreateEvent :!event OnGridGenerated))
  (EventDispatchers|BindEventtoOnOccupiedTileUpdated (Variables|Default|GetBP_Grid) (EventDispatchers|CreateEvent :!event OnTileDataUpdated))
  (Variables|Default|SetAC_TurnManager (Actor|GetComponentbyClass (Variables|Default|GetBP_Grid) "/Game/PF2e/Architecture/Combat/AC_TurnManager.AC_TurnManager_C"))
  (Input|EnableInput (Game|GetPlayerController 0)))

(event EventTick
  (params (DeltaSeconds :type Float%20%28single-precision%29))
  (CallFunction|UpdateTileUnderCursor))

(event Input|MouseEvents|DebugKeyLeftMouseButton
  (params (Key :type Key%20Structure :default "None") (ActionValue :type Input%20Action%20Value%20Structure))
  (bind _selectedaction_leftclick (Variables|ActionsAndInput|GetSelectedAction_LeftClick))
  (:Pressed
    (CallFunction|UpdateTileUnderCursor)
    (Variables|ActionsandInput|SetbIsLMBHeld true)
    (Utilities|IsValid _selectedaction_leftclick
      (:Is%20Valid
        (Default|ExecuteAction _selectedaction_leftclick (Variables|Default|GetHoveredTile)))))
  (:Released
    (Variables|ActionsandInput|SetbIsLMBHeld false)))

(event Input|MouseEvents|DebugKeyRightMouseButton
  (params (Key :type Key%20Structure :default "None") (ActionValue :type Input%20Action%20Value%20Structure))
  (bind _selectedaction_rightclick (Variables|ActionsAndInput|GetSelectedAction_RightClick))
  (:Pressed
    (CallFunction|UpdateTileUnderCursor)
    (Variables|ActionsandInput|SetbIsRMBHeld true)
    (Utilities|IsValid _selectedaction_rightclick
      (:Is%20Valid
        (Default|ExecuteAction _selectedaction_rightclick (Variables|Default|GetHoveredTile)))))
  (:Released
    (Variables|ActionsandInput|SetbIsRMBHeld false)))

(fn ConstructionScript)

(fn UpdateTileUnderCursor
  (Utilities|FlowControl|Sequence
    (:then_0
      (bind _hitactor (CallFunction|GetUnitUnderCursor))
      ;[0.15 0.15 0.15 0.5] SameDude?
      (if (!= (Variables|Default|GetHoveredUnitRef) _hitactor)
        (Utilities|FlowControl|Sequence
          (:then_0
            ;[0.15 0.15 0.15 0.5] UnhoverPreviousOne
            (Utilities|IsValid (Variables|Default|GetHoveredUnitRef) ; BeCarefulThereIsNoTestOnIfItsBP_Unit
              (:Is%20Valid
                (Class|BPIUnit|ChangeIsHovered(Message) (Variables|Default|GetHoveredUnitRef) false))))
          (:then_1
            ;[0.15 0.15 0.15 0.5] HoverNewOne
            (bind _output_get (Variables|Default|SetHoveredUnitRef _hitactor))
            (Utilities|IsValid _output_get
              (:Is%20Valid
                (Class|BPIUnit|ChangeIsHovered(Message) _output_get true)))))))
    (:then_1
      (Utilities|IsValid (Variables|Default|GetHoveredUnitRef)
        (:Is%20Valid
          (bind _newparam (Class|BPIUnit|GetIndex(Message) (Variables|Default|GetHoveredUnitRef)))
          (LocalVariables|SetNewIndex _newparam))
        (:Is%20Not%20Valid
          (bind _returnvalue (Class|Grid|GetTileIndexUnderCursor (Variables|Default|GetBP_Grid)))
          (LocalVariables|SetNewIndex _returnvalue)))
      (if (!= (LocalVariables|GetNewIndex) (Variables|Default|GetHoveredTile))
        (Default|RemoveStatefromTile (Variables|Default|GetBP_Grid) (Variables|Default|GetHoveredTile) "Hovered")
        (Variables|Default|SetHoveredTile (LocalVariables|GetNewIndex))
        (Default|AddStatetoTile (Variables|Default|GetBP_Grid) (Variables|Default|GetHoveredTile) "Hovered")
        (CallFunction|OnHoverTileChaged)))))

(fn SetSelectedActions
  (params (LeftAction :type BP%20Action%20Class%20Reference) (RightAction :type BP%20Action%20Class%20Reference))
  (Utilities|FlowControl|Sequence
    (:then_0
      (Utilities|IsValid (Variables|ActionsAndInput|GetSelectedAction_LeftClick)
        (:Is%20Valid
          (Actor|DestroyActor (Variables|ActionsAndInput|GetSelectedAction_LeftClick))
          (Variables|ActionsAndInput|SetSelectedAction_LeftClick 0))
        (:Is%20Not%20Valid
          _))
      (if (Utilities|IsValidClass LeftAction)
        (bind _returnvalue (Game|SpawnActorfromClass LeftAction (Math|Transform|MakeTransform "0, 0, 0" "0, 0, 0" "1.000000,1.000000,1.000000") "AlwaysSpawn" "MultiplyWithRoot" 0 self 0))
        (Variables|ActionsAndInput|SetSelectedAction_LeftClick _returnvalue)))
    (:then_1
      (Utilities|IsValid (Variables|ActionsAndInput|GetSelectedAction_RightClick)
        (:Is%20Valid
          (Actor|DestroyActor (Variables|ActionsAndInput|GetSelectedAction_RightClick))
          (Variables|ActionsAndInput|SetSelectedAction_RightClick 0))
        (:Is%20Not%20Valid
          _))
      (if (Utilities|IsValidClass RightAction)
        (bind _returnvalue_2 (Game|SpawnActorfromClass RightAction (Math|Transform|MakeTransform "0, 0, 0" "0, 0, 0" "1.000000,1.000000,1.000000") "AlwaysSpawn" "MultiplyWithRoot" 0 self 0))
        (Variables|ActionsAndInput|SetSelectedAction_RightClick _returnvalue_2)))
    (:then_2
      (Default|CallOnSelectedActorsChanged (Variables|ActionsAndInput|GetSelectedAction_LeftClick) (Variables|ActionsAndInput|GetSelectedAction_RightClick)))))

(fn GetUnitUnderCursor
  (bind _returnvalue (Game|GetPlayerController 0))
  (bind _bp_grid (Variables|Default|GetBP_Grid))
  (bind (_hitresult _returnvalue_2) (Game|Player|GetHitResultUnderCursorbyChannel _returnvalue "TraceTypeQuery5" true))
  (if _returnvalue_2
    (return (.HitActor (Collision|BreakHitResult _hitresult)))
    (else
      (bind _returnvalue_3 (Class|Grid|GetTileIndexUnderCursor _bp_grid))
      (return (Utilities|Struct|BreakS_TileData (.Value (Utilities|Map|Find (Variables|/Game/PF2e/Architecture/Grid/BP_Grid.BP_Grid_C|GetGridTiles _bp_grid) _returnvalue_3)))))))

(fn SetSelectedTileandUnit
  (params (Index :type Int%20Point%20Structure) (force :type Boolean))
  (Utilities|FlowControl|Sequence
    (:then_0
      ;[0.15 0.15 0.15 0.5] SeletingTIle
      (if (or (!= Index (Variables|Default|GetSelectedTile)) force)
        (Default|RemoveStatefromTile (Variables|Default|GetBP_Grid) (Variables|Default|GetSelectedTile) "Selected")
        (Variables|Default|SetSelectedTile Index)
        (Default|AddStatetoTile (Variables|Default|GetBP_Grid) (Variables|Default|GetSelectedTile) "Selected")
        (else
          (Default|RemoveStatefromTile (Variables|Default|GetBP_Grid) (Variables|Default|GetSelectedTile) "Selected")
          (Variables|Default|SetSelectedTile (Utilities|Struct|MakeIntPoint -1000 -1000))))
      (Default|CallOnSelectedTileChanged (Variables|Default|GetSelectedTile)))
    (:then_1
      ;[0.15 0.15 0.15 0.5] SelectingUnit
      (LocalVariables|SetNewUnit (.AsBP%20Unit (Utilities|Casting|CastToBP_Unit (.UnitOnTile (Utilities|Struct|BreakS_TileData (.Value (Utilities|Map|Find (Variables|/Game/PF2e/Architecture/Grid/BP_Grid.BP_Grid_C|GetGridTiles (Variables|Default|GetBP_Grid)) (Variables|Default|GetSelectedTile))))))))
      (if (or (!= (Variables|Default|GetSelectedUnitRef) (LocalVariables|GetNewUnit)) force)
        (Utilities|FlowControl|Sequence
          (:then_0
            ;;[0.15 0.15 0.15 0.5] Unselect
            (Utilities|IsValid (Variables|Default|GetSelectedUnitRef) ; BeCarefulThereIsNoTestOnIfItsBP_Unit
              (:Is%20Valid
                (Default|SetIsSelected (Variables|Default|GetSelectedUnitRef) false))))
          (:then_1
            ;;[0.15 0.15 0.15 0.5] Select
            (bind _output_get (Variables|Default|SetSelectedUnitRef (LocalVariables|GetNewUnit)))
            (Utilities|IsValid _output_get
              (:Is%20Valid
                (Default|SetIsSelected _output_get true)))))))))

(fn OnGridGenerated
  (if (Class|Grid|IsIndexValid (Variables|Default|GetBP_Grid) (Variables|Default|GetSelectedTile))
    (CallFunction|SetSelectedTileandUnit (Variables|Default|GetSelectedTile) true)
    (else
      (CallFunction|SetSelectedTileandUnit (Utilities|Struct|MakeIntPoint -999 0) false))))

(fn OnTileDataUpdated
  (params (Index :type Int%20Point%20Structure))
  (if (Class|KismetMathLibrary|EqualIntPointIntPoint Index (Variables|Default|GetSelectedTile))
    (CallFunction|OnGridGenerated)))

(fn OnUnitGridIndexChange
  (params (Unit :type BP%20Unit%20Object%20Reference))
  (if (== (Variables|Default|GetSelectedUnitRef) Unit)
    (CallFunction|SetSelectedTileandUnit (Variables|/Game/PF2e/Units/BP_Unit.BP_Unit_C|GetLocationIndex Unit) false)))