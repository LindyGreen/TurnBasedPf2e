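; AC_UnitData is a component that stores a unit's data struct, including its stats, for the PF2e game.
; It exposes a setter and getter for the whole struct, a getter for the nested stats, and a setter that edits only the move duration per tile within those stats.
; The event graph is empty, so the component only holds and serves data.
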(event EventBeginPlay)

(event EventTick
  (params (DeltaSeconds :type Float%20%28single-precision%29)))

(fn SetUnitData
  (params (Input :type S%20Unit%20Data%20Structure))
  (Variables|Default|SetUnitData Input))

(fn GetUnitData
  (return (Variables|Default|GetUnitData)))

(fn GetUnitStats
  (return (.Stats (Utilities|Struct|BreakS_UnitData (Variables|Default|GetUnitData)))))

(fn SetMoveDurationPerTile
  (params (Stats%20Move%20Duration%20Per%20Tile :type Float%20%28double-precision%29))
  (Utilities|Struct|SetmembersinS_UnitDataStats (.Stats (Utilities|Struct|BreakS_UnitData (Variables|Default|GetUnitData))) Stats%20Move%20Duration%20Per%20Tile))