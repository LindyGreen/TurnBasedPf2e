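; BP_GridSpawner is a placed actor that spawns a BP_Grid at its own transform on a debug Space Bar press.
; It enables player input on BeginPlay, and a Blocker flag limits the spawn to a single attempt.
; The press async-loads the GridRef class, passes tile counts and an enemy row name into the new grid, then notifies the player controller through GridWasSpawnedMessage.
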(event EventBeginPlay
  (Input|EnableInput (Game|GetPlayerController 0)))

(event Collision|EventActorBeginOverlap
  (params (OtherActor :type Actor%20Object%20Reference)))

(event EventTick
  (params (DeltaSeconds :type Float%20%28single-precision%29)))

(event Input|KeyboardEvents|DebugKeySpaceBar
  (params (Key :type Key%20Structure :default "None") (ActionValue :type Input%20Action%20Value%20Structure))
  (:Pressed
    (if (not (Variables|Default|GetBlocker))
      (Variables|Default|SetBlocker true)
      (bind _class (Utilities|AsyncLoadClassAsset (Variables|Default|GetGridRef))
        (:Completed
          (bind _asbp_grid (Utilities|Casting|CastToBP_GridClass _class))
          (bind _returnvalue (Game|SpawnActorfromClass :Class _asbp_grid :SpawnTransform (Transformation|GetActorTransform) :CollisionHandlingOverride "AdjustIfPossibleButAlwaysSpawn" :TransformScaleMethod "MultiplyWithRoot" :TileCountX (Variables|Default|GetTileCountX) :TileCountY (Variables|Default|GetTileCountY) :EnemiesOnMapRowName (Variables|Default|GetEnemies%20on%20Map%20Row%20Name) :Instigator 0))
          (Class|BPIPlayerController|GridWasSpawned(Message) (Game|GetPlayerController 0) _returnvalue))))))

(fn ConstructionScript)